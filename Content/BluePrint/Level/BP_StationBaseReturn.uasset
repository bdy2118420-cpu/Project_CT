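; BP_StationBaseReturn is the cooking game's return station, where a chef hands in a plate to fulfil active orders.
; On InteractPress, if the held item's name contains "접시" (plate), GetItemDatas looks up the GameMode's active orders in DT_ItemData.
; Name matches remove the order, call CallOrder and SuccessOrder, then destroy the item taken from the chef.
; FailedOrder depends on a Failed flag, cleared on successful hand-in and never reset here.
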(event `self.ReceiveBeginPlay`
  (`parent.ReceiveBeginPlay`)
  (bind _asbp_gamemode_cook (cast `/Game/BluePrint/Core/BP_GamemodeCook` (`GameplayStatics.GetGameMode`)))
  (set `self.As BP Gamemode Cook` _asbp_gamemode_cook))

(event `/Game/Interfaces/BPI_Interactable.InteractPress`
  (params (Interactor :type "Actor Object Reference"))
  (bind (_orderarray_order_id _orderarray_mainicon _orderarray_ingredienticons _orderarray_currenttime) (break `/Game/Data/ST_Order` (`self.OrderArray`)))
  (bind _as_bp_gamemode_cook (`self.As BP Gamemode Cook`))
  (bind _activeorders (`/Game/BluePrint/Core/BP_GamemodeCook.ActiveOrders` (`self.As BP Gamemode Cook`)))
  (bind _itemdata_itemname (break `/Game/Data/ST_ItemData` (`/Game/BluePrint/Item/BP_ItemBase.ItemData` (`/Game/BluePrint/Core/BP_Chef.CurrentHeldItem` (`self.As BP Chef`)))))
  (bind _output_get (set `self.Interactor` Interactor))
  (bind _asbp_chef (cast `/Game/BluePrint/Core/BP_Chef` _output_get))
  (set `self.As BP Chef` _asbp_chef)
  (if (`KismetStringLibrary.Contains` _itemdata_itemname "접시")
    (`self.GetItemDatas`)
    (bind _asbp_plate (cast `/Game/BluePrint/Item/BP_Plate` (`/Game/BluePrint/Core/BP_Chef.CurrentHeldItem` (`self.As BP Chef`))))
    (set `self.As BP Plate` _asbp_plate)
    (for (_array_element _array_index) (`self.Item`)
      (`/Engine/EditorBlueprintResources/StandardMacros.IsValid` (`self.As BP Plate`)
        (:`Is Valid`
          (if (== (`.ItemName_10_2055E54645D7D841E4D9E4863A9F20C6` (break `/Game/Data/ST_ItemData` _array_element)) (`.ItemName_10_2055E54645D7D841E4D9E4863A9F20C6` (break `/Game/Data/ST_ItemData` (`/Game/BluePrint/Item/BP_Plate.Item Info` (`self.As BP Plate`)))))
            (set `self.OrderArray` (`|GetArrayItem` _activeorders _array_index))
            (`KismetArrayLibrary.Array_Remove` _activeorders _array_index)
            (`/Game/BluePrint/Core/BP_GamemodeCook.Order` _as_bp_gamemode_cook)
            (`/Game/BluePrint/Core/BP_GamemodeCook.SuccessOrder` _as_bp_gamemode_cook _orderarray_currenttime)
            (bind (_issuccess _iteminfo _actorinfo) (message `/Game/Interfaces/BPI_ItemHandler.TakeItem` (`self.Interactor`)))
            (`/Engine/EditorBlueprintResources/StandardMacros.IsValid` _actorinfo
              (:`Is Valid`
                (`self.K2_DestroyActor` _actorinfo)
                (set `self.Failed` false)))))))
    (if (`self.Failed`)
      (`/Game/BluePrint/Core/BP_GamemodeCook.FailedOrder` (`self.As BP Gamemode Cook`) 0.0))))

(fn `GetItemDatas`
  (`KismetArrayLibrary.Array_Clear` (`self.Item`))
  (for _array_element (`/Game/BluePrint/Core/BP_GamemodeCook.ActiveOrders` (`self.As BP Gamemode Cook`))
    (bind _returnvalue (`|GetDataTableRow` "/Game/Data/DT_ItemData.DT_ItemData" (`.Order_Id_2_AFE16D9F40B8A59230639FB7680B77DC` (break `/Game/Data/ST_Order` _array_element)))
      (:`then`
        (`KismetArrayLibrary.Array_Add` (`self.Item`) _returnvalue)))))

(fn `UserConstructionScript`
  (`parent.UserConstructionScript`))