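; Cutting board station in a cooking game where a chef places an ingredient, cuts it and collects the result.
; Placing a matching item attaches it to a socket and looks up output and cook time in the recipe DataTable by ingredient and station.
; Holding interact freezes the chef and enables Tick to fill a progress widget, and releasing pauses it.
; CutDone swaps the ingredient for a spawned output item built from the item DataTable.
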(event `self.ReceiveBeginPlay`
  (`parent.ReceiveBeginPlay`)
  (bind _aswbp_progress (cast `/Game/UI/WBP_Progress` (`WidgetComponent.GetUserWidgetObject` (`self.Widget`))))
  (set `self.As WBP Cuting Progress` _aswbp_progress))

(event `self.ReceiveTick`
  (params (DeltaSeconds :type "Float (single-precision)"))
  (`parent.ReceiveTick` DeltaSeconds)
  (`self.SetProgress`))

(event `CustomEvent_0`
  ; 커팅 완료시 진행
  (`self.DoneSetting`)
  (`self.SetReturnItem`))

(event `/Game/Interfaces/BPI_Interactable.InteractPress`
  (params (Interactor :type "Actor Object Reference"))
  (bind _bp_chef (`self.BP_Chef`))
  (bind _output_get (set `self.Interactor` Interactor))
  (bind _asbp_chef (cast `/Game/BluePrint/Core/BP_Chef` _output_get))
  (set `self.BP_Chef` _asbp_chef)
  ; 도마에 아이템이 없을때
  (`/Engine/EditorBlueprintResources/StandardMacros.IsValid` (`self.HeldItem`)
    (:`Is Valid`
      ; 현재 커팅중인지
      (if (`self.IsProcessing`)
        (set `CharacterMovementComponent.MaxWalkSpeed` 0.0 (`Character.CharacterMovement` _bp_chef))
        (`/Game/BluePrint/Core/BP_Chef.Cut` _bp_chef)
        (`self.SetActorTickEnabled` true)
        (add `self.CutDone` (delegate `CustomEvent_0`))
        (else
          ; 아이템 회수
          (`self.GetItem`))))
    (:`Is Not Valid`
      (`self.SpawnItem`))))

(event `/Game/Interfaces/BPI_Interactable.InteractUnPress`
  (params (Interactor :type "Actor Object Reference"))
  (bind _bp_chef (`self.BP_Chef`))
  ; 버튼 땠을때
  (`/Engine/EditorBlueprintResources/StandardMacros.IsValid` _bp_chef
    (:`Is Valid`
      (set `CharacterMovementComponent.MaxWalkSpeed` 600.0 (`Character.CharacterMovement` _bp_chef))
      (`/Game/BluePrint/Core/BP_Chef.Cut` _bp_chef)
      (`self.SetActorTickEnabled` false))))

(fn `DoneSetting`
  (set `self.IsProcessing` false)
  ; 작업 완료시 ui숨김 플레이어 애니메이션 정지, ui 퍼센트 초기화
  (set `self.CurrentProgress` 0.0)
  (set `self.Time` 0.0)
  (`/Game/Interfaces/BPI_Interactable.InteractUnPress` null)
  (`SceneComponent.SetVisibility` (`self.Widget`) false false)
  (`self.K2_DestroyActor` (`self.HeldItem`)))

(fn `FindRecipe`
  (returns (OutputItem :type String) (Cookingtime :type "Float (double-precision)"))
  (locals (NewLocalVar :type "Array of Name"))
  (bind _currentitemdata_itemname (break `/Game/Data/ST_ItemData` (`self.CurrentItemData`)))
  (bind _outrownames (`DataTableFunctionLibrary.GetDataTableRowNames` "/Game/Data/DT_RecipeData.DT_RecipeData"))
  (bind _output_get (set `local.NewLocalVar` _outrownames))
  (for _array_element _output_get
    (bind _returnvalue (`|GetDataTableRow` "/Game/Data/DT_RecipeData.DT_RecipeData" _array_element)
      (:`then`
        (if (and (`KismetArrayLibrary.Array_Contains` (break `/Game/Data/ST_Recipe` _returnvalue) _currentitemdata_itemname) (== (`.RequiredStation_15_995D9C9146BBD48278CB90BE966B2076` (break `/Game/Data/ST_Recipe` _returnvalue)) (`self.StationID`)))
          (return (`.OutputItem_5_E6AE20634EA5909F58B832BF1A9DF584` (break `/Game/Data/ST_Recipe` _returnvalue)) (`.Cookingtime_11_9CDD3667464780268DD0E387204BF1B4` (break `/Game/Data/ST_Recipe` _returnvalue))))))))

(fn `GetItem`
  (bind _itemdata_itemname (break `/Game/Data/ST_ItemData` (`/Game/BluePrint/Item/BP_ItemBase.ItemData` (`/Game/BluePrint/Core/BP_Chef.CurrentHeldItem` (`self.BP_Chef`)))))
  ; 이미 다른 아이템을 들고있으면 회수 불가능
  (`/Engine/EditorBlueprintResources/StandardMacros.IsValid` (`/Game/BluePrint/Core/BP_Chef.CurrentHeldItem` (`self.BP_Chef`))
    (:`Is Valid`
      (if (`KismetStringLibrary.Contains` _itemdata_itemname "접시")
        (message `/Game/Interfaces/BPI_ItemHandler.GiveItem` (`self.Interactor`) (`self.CurrentItemData`) (`self.HeldItem`))))
    (:`Is Not Valid`
      (message `/Game/Interfaces/BPI_ItemHandler.GiveItem` (`self.Interactor`) (`self.CurrentItemData`) (`self.HeldItem`))
      (set `self.HeldItem` null))))

(fn `SetProgress`
  ; 틱마다 진행 경과를 계산하고 ui갱신
  (bind _output_get (set `self.Time` (+ (`GameplayStatics.GetWorldDeltaSeconds`) (`self.Time`))))
  (bind _output_get_2 (set `self.CurrentProgress` (/ _output_get (`self.Cookingtime`))))
  (`ProgressBar.SetPercent` (`/Game/UI/WBP_Progress.CutProgress` (`self.As WBP Cuting Progress`)) _output_get_2)
  (if (>= _output_get_2 (`self.DoneProgress`))
    (`self.CutDone`)))

(fn `SetRecipe`
  (set `self.IsProcessing` true)
  (`SceneComponent.SetVisibility` (`self.Widget`) true false)
  (bind (_outputitem _cookingtime) (`self.FindRecipe`))
  (set `self.Output Item` _outputitem)
  (set `self.Cookingtime` _cookingtime))

(fn `SetReturnItem`
  (bind _returnvalue (`|GetDataTableRow` "/Game/Data/DT_ItemData.DT_ItemData" (`KismetStringLibrary.Conv_StringToName` (`self.Output Item`)))
    (:`then`
      (bind _output_get (set `self.CurrentItemData` _returnvalue))
      (bind _returnvalue_2 (`|SpawnActorFromClass` "/Game/BluePrint/Item/BP_ItemBase.BP_ItemBase_C" (`SceneComponent.GetSocketTransform` (`self.StaticMesh`) "FoodCounter" "RTS_World") "Undefined" "MultiplyWithRoot" null null))
      (set `self.HeldItem` _returnvalue_2)
      (set `/Game/BluePrint/Item/BP_ItemBase.ItemData` (`self.CurrentItemData`) _returnvalue_2)
      (`StaticMeshComponent.SetStaticMesh` (`/Game/BluePrint/Item/BP_ItemBase.StaticMesh` _returnvalue_2) (`.Item3DModel_18_8779E8244BCBF5E4A785AB940C4C2424` (break `/Game/Data/ST_ItemData` _output_get))))))

(fn `SpawnActorOnCutBoard`
  (params (Interactor :type "Object Object Reference"))
  (bind (_issuccess _iteminfo _actorinfo) (message `/Game/Interfaces/BPI_ItemHandler.TakeItem` Interactor))
  (set `self.CurrentItemData` _iteminfo)
  (if _issuccess
    (bind _output_get (set `self.HeldItem` _actorinfo))
    (`self.K2_AttachToComponent` _output_get (`self.StaticMesh`) "FoodCounter" "SnapToTarget" "SnapToTarget" "KeepWorld" true)))

(fn `SpawnItem`
  (bind (_currentitemdata_itemname _currentitemdata_itemicon _currentitemdata_item3dmodel _currentitemdata_requiredstation) (break `/Game/Data/ST_ItemData` (`/Game/BluePrint/Core/BP_Chef.CurrentItemData` (`self.BP_Chef`))))
  ; 도마위의 없으면 머리위의 아이템 소환
  (if (== _currentitemdata_requiredstation (`self.StationID`))
    (`self.SpawnActorOnCutBoard` (`self.Interactor`))
    (`self.SetRecipe`)
    (return)))

(fn `UserConstructionScript`
  (`parent.UserConstructionScript`))