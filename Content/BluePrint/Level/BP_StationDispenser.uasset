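; BP_StationDispenser is a kitchen station that hands a new item to an empty-handed chef on interact.
; Its construction script sets the station mesh from the dispenser data table row matching DispenseID.
; On interact, that row's target ID looks up item data, spawning a plate if the name contains "접시" (plate), otherwise a base item.
; The spawned item receives its mesh and data, then goes to the chef via GiveItemMessage.
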(event `/Game/Interfaces/BPI_Interactable.InteractPress`
  (params (Interactor :type "Actor Object Reference"))
  (bind _output_get (set `self.Interactor` Interactor))
  (bind _asbp_chef (cast `/Game/BluePrint/Core/BP_Chef` _output_get))
  (`/Engine/EditorBlueprintResources/StandardMacros.IsValid` (`/Game/BluePrint/Core/BP_Chef.CurrentHeldItem` _asbp_chef)
    (:`Is Not Valid`
      (bind _output_get_2 (`self.GetItemData` _asbp_chef))
      (`self.SetMesh` _output_get_2))))

(fn `GetItemData`
  (params (self2 :type "/Game/BluePrint/Core/BP_Chef Object Reference"))
  (returns (Output_Get :type "/Game/BluePrint/Item/BP_ItemBase Object Reference"))
  ; 상호작용 발생시 자기 자신의 Actor정보를 데이터 테이블에서 찾아 넘겨줌
  (`/Engine/EditorBlueprintResources/StandardMacros.IsValid` (`/Game/BluePrint/Core/BP_Chef.CurrentHeldItem` self2)
    (:`Is Not Valid`
      (bind _returnvalue (`|GetDataTableRow` "/Game/Data/DT_DIspenserData.DT_DIspenserData" (`self.DispenseID`))
        (:`then`
          (bind _returnvalue_2 (`|GetDataTableRow` "/Game/Data/DT_ItemData.DT_ItemData" (`.TargetItemID_9_9878566A4187DF66ADACBC95CD162081` (break `/Game/Data/ST_DIspenserData` _returnvalue)))
            (:`then`
              (bind _output_get (set `self.Out Row` _returnvalue_2))
              (bind _returnvalue_3 (`|SpawnActorFromClass` (select `bool` (`KismetStringLibrary.Contains` (break `/Game/Data/ST_ItemData` _output_get) "접시") :`false` "/Game/BluePrint/Item/BP_ItemBase.BP_ItemBase_C" :`true` "/Game/BluePrint/Item/BP_Plate.BP_Plate_C" :!type "Actor Class Reference") (`self.GetTransform`) "Undefined" "MultiplyWithRoot" null null))
              (bind _asbp_item_base (cast `/Game/BluePrint/Item/BP_ItemBase` _returnvalue_3))
              (bind _output_get_2 (set `self.Return` _asbp_item_base)))
            (:`RowNotFound`
              _))
          (return _output_get_2))))))

(fn `SetMesh`
  (params (self2 :type "/Game/BluePrint/Item/BP_ItemBase Object Reference"))
  (bind (_out_row_itemname _out_row_itemicon _out_row_item3dmodel) (break `/Game/Data/ST_ItemData` (`self.Out Row`)))
  (`/Engine/EditorBlueprintResources/StandardMacros.IsValid` self2
    (:`Is Valid`
      (`StaticMeshComponent.SetStaticMesh` (`/Game/BluePrint/Item/BP_ItemBase.StaticMesh` self2) _out_row_item3dmodel)
      (set `/Game/BluePrint/Item/BP_ItemBase.ItemData` (`self.Out Row`) (`self.Return`))
      (message `/Game/Interfaces/BPI_ItemHandler.GiveItem` (`self.Interactor`) (`self.Out Row`) (`self.Return`)))))

(fn `UserConstructionScript`
  ; ID에 따른 Mesh변환
  (`parent.UserConstructionScript`)
  (bind _returnvalue (`|GetDataTableRow` "/Game/Data/DT_DIspenserData.DT_DIspenserData" (`self.DispenseID`))
    (:`then`
      (bind _output_get (set `self.ST_Dispense` _returnvalue))
      (`StaticMeshComponent.SetStaticMesh` (`self.StaticMesh`) (`.StationMesh_12_095537A74EC48472C8B823A21282EC04` (break `/Game/Data/ST_DIspenserData` _output_get))))))