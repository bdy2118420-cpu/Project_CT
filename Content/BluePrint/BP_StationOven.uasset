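; Oven cooking station that takes a chef's held item, cooks it over time and burns it if left too long.
; Interaction accepts items matching its StationID, looks up output and cook time in DT_RecipeData, and enables Tick.
; Tick fills cook, then red overcook progress widgets, firing Done and OverCook dispatchers that swap in the cooked item, or trash plus Niagara flame.
; An empty-handed chef collects the result, resetting the station.
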(event `self.ReceiveBeginPlay`
  (`parent.ReceiveBeginPlay`)
  (`self.SetUI`))

(event `self.ReceiveTick`
  (params (DeltaSeconds :type "Float (single-precision)"))
  (`parent.ReceiveTick` DeltaSeconds)
  (if (not (`self.IsCookDone`))
    ; 조리중
    (`self.CookProgress`)
    (else
      ; 조리 완료부터 오버쿡까지
      (`self.OverCookProgress`))))

(event `/Game/Interfaces/BPI_Interactable.InteractPress`
  (params (Interactor :type "Actor Object Reference"))
  (bind (_currentitemdata_itemname _currentitemdata_itemicon _currentitemdata_item3dmodel _currentitemdata_requiredstation) (break `/Game/Data/ST_ItemData` (`/Game/BluePrint/BP_Chef.CurrentItemData` (`self.As BP Chef`))))
  (bind _output_get (set `self.Interactor` Interactor))
  (bind _asbp_chef (cast `/Game/BluePrint/BP_Chef` _output_get))
  (set `self.As BP Chef` _asbp_chef)
  ; 요리 완료 밑 플레이어가 아무것도 안가지고 있을때
  ;; 조리중일때
  (if (`self.IsProcessing`)
    (if (`self.IsCookDone`)
      (`/Engine/EditorBlueprintResources/StandardMacros.IsValid` (`/Game/BluePrint/BP_Chef.CurrentHeldItem` (`self.As BP Chef`))
        (:`Is Not Valid`
          (`/Game/BluePrint/BP_Chef.GiveItem` (`self.As BP Chef`) (`self.CurrentItemData`))
          (`self.SetCookDone`))))
    (elif (== _currentitemdata_requiredstation (`self.StationID`))
      ; 조리중이 아니고 아무아이템도 없으면 가져오기
      (`/Engine/EditorBlueprintResources/StandardMacros.IsValid` (`/Game/BluePrint/BP_Chef.CurrentHeldItem` (`self.As BP Chef`))
        (:`Is Valid`
          (bind (_issuccess _iteminfo) (message `/Game/Interfaces/BPI_ItemHandler.TakeItem` (`self.Interactor`)))
          (set `self.CurrentItemData` _iteminfo)
          ; 레시피 세팅
          (bind (_outputitem _cookingtime) (`self.SetRecipe`))
          (set `self.Output Item` _outputitem)
          (set `self.Cookingtime` _cookingtime)
          (set `self.IsProcessing` true)
          ; 요리완료와 오버쿡 이벤트 바인드
          (add `self.Done` (delegate `CookDone`))
          (add `self.OverCook` (delegate `OverCookDone`))
          ; 시간계산 시작, UI보이게
          (`self.SetActorTickEnabled` true)
          (`SceneComponent.SetVisibility` (`self.Widget`) true false)
          (`SceneComponent.SetVisibility` (`self.Widget1`) true false))))))

(event `CookDone`
  (set `self.IsCookDone` true)
  (bind _returnvalue (`|GetDataTableRow` "/Game/Data/DT_ItemData.DT_ItemData" (`KismetStringLibrary.Conv_StringToName` (`self.Output Item`)))
    (:`then`
      (set `self.CurrentItemData` _returnvalue))))

(event `OverCookDone`
  (bind (_returnvalue_x _returnvalue_y _returnvalue_z) (`KismetMathLibrary.BreakVector` (`self.K2_GetActorLocation`)))
  (`self.SetActorTickEnabled` false)
  (bind _returnvalue (`|GetDataTableRow` "/Game/Data/DT_ItemData.DT_ItemData" "Item_Trash")
    (:`then`
      (set `self.CurrentItemData` _returnvalue)
      (bind _returnvalue_2 (`NiagaraFunctionLibrary.SpawnSystemAtLocation` "/Game/F_FreeFlameFx_Pack/FX/NS_Flame_4.NS_Flame_4" (`KismetMathLibrary.MakeVector` _returnvalue_x _returnvalue_y (+ _returnvalue_z 50.0)) (struct) (1.2 1.2 1.2)))
      (set `self.Fire` _returnvalue_2))))

(fn `CookProgress`
  (bind _output_get (`self.GetProgress`))
  (`ProgressBar.SetPercent` (`/Game/UI/WBP_Progress.CutProgress` (`self.As WBP Progress`)) _output_get)
  (if (>= _output_get (`self.DoneProgress`))
    (`self.Done`)))

(fn `GetProgress`
  (returns (Output_Get :type "Float (double-precision)"))
  (set `self.Time` (+ (`GameplayStatics.GetWorldDeltaSeconds`) (`self.Time`)))
  (bind _output_get (set `self.CurrentProgress` (/ (`self.Time`) (`self.Cookingtime`))))
  (return _output_get))

(fn `OverCookProgress`
  (bind _output_get (`self.GetProgress`))
  (`ProgressBar.SetPercent` (`/Game/UI/WBP_Progress.CutProgress` (`self.As WBP ProgressOverCook`)) (- _output_get 1.0))
  (if (>= _output_get (* (`self.DoneProgress`) 2.0))
    (`self.OverCook`)))

(fn `SetCookDone`
  (bind _fire (`self.Fire`))
  (set `self.CurrentItemData` (struct))
  (set `self.IsProcessing` false)
  (set `self.IsCookDone` false)
  (set `self.Time` 0.0)
  (set `self.CurrentProgress` 0.0)
  (`self.SetActorTickEnabled` false)
  (`ProgressBar.SetPercent` (`/Game/UI/WBP_Progress.CutProgress` (`self.As WBP Progress`)) 0.0)
  (`ProgressBar.SetPercent` (`/Game/UI/WBP_Progress.CutProgress` (`self.As WBP ProgressOverCook`)) 0.0)
  (`SceneComponent.SetVisibility` (`self.Widget`) false false)
  (`SceneComponent.SetVisibility` (`self.Widget1`) false false)
  (`SceneComponent.K2_DetachFromComponent` _fire "KeepRelative" "KeepRelative" "KeepRelative" true)
  (`ActorComponent.K2_DestroyComponent` _fire))

(fn `SetRecipe`
  (returns (OutputItem :type String) (Cookingtime :type "Float (double-precision)"))
  (locals (NewLocalVar :type "Array of Name"))
  (bind _currentitemdata_itemname (break `/Game/Data/ST_ItemData` (`self.CurrentItemData`)))
  (bind _outrownames (`DataTableFunctionLibrary.GetDataTableRowNames` "/Game/Data/DT_RecipeData.DT_RecipeData"))
  (bind _output_get (set `local.NewLocalVar` _outrownames))
  (for _array_element _output_get
    (bind _returnvalue (`|GetDataTableRow` "/Game/Data/DT_RecipeData.DT_RecipeData" _array_element)
      (:`then`
        (if (and (`KismetArrayLibrary.Array_Contains` (break `/Game/Data/ST_Recipe` _returnvalue) _currentitemdata_itemname) (== (`.RequiredStation_15_995D9C9146BBD48278CB90BE966B2076` (break `/Game/Data/ST_Recipe` _returnvalue)) (`self.StationID`)))
          (return (`.OutputItem_5_E6AE20634EA5909F58B832BF1A9DF584` (break `/Game/Data/ST_Recipe` _returnvalue)) (`.Cookingtime_11_9CDD3667464780268DD0E387204BF1B4` (break `/Game/Data/ST_Recipe` _returnvalue))))))))

(fn `SetUI`
  (bind _aswbp_progress (cast `/Game/UI/WBP_Progress` (`WidgetComponent.GetUserWidgetObject` (`self.Widget`))))
  (set `self.As WBP Progress` _aswbp_progress)
  (bind _aswbp_progress_2 (cast `/Game/UI/WBP_Progress` (`WidgetComponent.GetUserWidgetObject` (`self.Widget1`))))
  (bind _output_get (set `self.As WBP ProgressOverCook` _aswbp_progress_2))
  (`ProgressBar.SetFillColorAndOpacity` (`/Game/UI/WBP_Progress.CutProgress` _output_get) (struct :`R` 1.0 :`A` 1.0)))

(fn `UserConstructionScript`
  (`parent.UserConstructionScript`))