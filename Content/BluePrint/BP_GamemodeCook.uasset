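; Cooking game mode that creates the main HUD and fills it with random dish orders.
; On BeginPlay it builds the dish pool from DT_ItemData rows whose required station is Station_Return, then starts a looping timer with a random interval picked once.
; Each tick puts a random dish icon in the first empty of six HUD borders and records the order.
; SubmitDish and the Failed handler are stubs.
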(event `self.ReceiveBeginPlay`
  (`self.SetDishes`)
  (bind _returnvalue (`|CreateWidget` "/Game/UI/WBP_Main.WBP_Main_C" (`GameplayStatics.GetPlayerController` 0)))
  (bind _output_get (set `self.MainUI` _returnvalue))
  (`UserWidget.AddToViewport` _output_get 0)
  (bind _output_get_2 (set `self.Randomtime` (`KismetMathLibrary.Conv_IntToDouble` (`KismetMathLibrary.RandomIntegerInRange` 1 5))))
  (`KismetSystemLibrary.K2_SetTimerDelegate` (delegate `CustomEvent`) _output_get_2 true true)
  (add `self.Faild` (delegate `Failed`)))

(event `Failed`)

(event `CustomEvent`
  (`self.SetUi`)
  (set `self.Randomtime` (`KismetMathLibrary.Conv_IntToDouble` (`KismetMathLibrary.RandomIntegerInRange` 1 5))))

(fn `GetRandomDish`
  (`KismetArrayLibrary.Array_Add` (`self.OrderDishes`) (`KismetArrayLibrary.Array_Random` (`self.Dishes`))))

(fn `SetDishes`
  (locals (NewLocalVar :type "/Game/Data/ST_ItemData Structure") (Name :type Name))
  (`KismetArrayLibrary.Array_Clear` (`self.OrderDishes`))
  (`KismetArrayLibrary.Array_Clear` (`self.Dishes`))
  (bind _outrownames (`DataTableFunctionLibrary.GetDataTableRowNames` "/Game/Data/DT_ItemData.DT_ItemData"))
  (for _array_element _outrownames
    (set `local.Name` _array_element)
    (bind _returnvalue (`|GetDataTableRow` "/Game/Data/DT_ItemData.DT_ItemData" _array_element)
      (:`then`
        (bind _output_get (set `local.NewLocalVar` _returnvalue))
        (if (== (`.RequiredStation_23_9146ECD94E0ADE84DA6122B02AA0D29B` (break `/Game/Data/ST_ItemData` _output_get)) "Station_Return")
          (`KismetArrayLibrary.Array_Add` (`self.Dishes`) (`local.NewLocalVar`))
          (`KismetArrayLibrary.Array_Add` (`self.DishNames`) (`local.Name`)))))))

(fn `SetOrderUi`
  (params (UI :type "/Game/UI/WBP_OrderIcon Object Reference") (WidgetNum :type Integer))
  (locals (OrderDish :type "/Game/Data/ST_ItemData Structure") (NewLocalVar_0 :type Integer :default 0))
  (bind (_output_itemname _output_itemicon) (break `/Game/Data/ST_ItemData` (`|GetArrayItem` (`self.Dishes`) (`local.NewLocalVar_0`))))
  (set `local.NewLocalVar_0` (`.OutIndex` (`KismetArrayLibrary.Array_Random` (`self.Dishes`))))
  (`Image.SetBrushFromTexture` (`/Game/UI/WBP_OrderIcon.FoodIcon` (`local.UI`)) _output_itemicon true)
  (`KismetArrayLibrary.Array_Add` (`self.OrderDishes`) (`|GetArrayItem` (`self.Dishes`) (`local.NewLocalVar_0`)))
  (set `/Game/UI/WBP_OrderIcon.RecipName` (`|GetArrayItem` (`self.DishNames`) (`local.NewLocalVar_0`)) (`local.UI`)))

(fn `SetUi`
  (bind _mainui (`self.MainUI`))
  (bind _output_get (set `self.Borders` (`|MakeArray` (`/Game/UI/WBP_Main.Border_0` _mainui) (`/Game/UI/WBP_Main.Border_1` _mainui) (`/Game/UI/WBP_Main.Border_2` _mainui) (`/Game/UI/WBP_Main.Border_3` _mainui) (`/Game/UI/WBP_Main.Border_4` _mainui) (`/Game/UI/WBP_Main.Border_5` _mainui))))
  (for _array_element _output_get
    (bind _asborder (cast `Border` _array_element))
    (if (not (`PanelWidget.HasAnyChildren` _asborder))
      (bind _returnvalue (`|CreateWidget` "/Game/UI/WBP_OrderIcon.WBP_OrderIcon_C"))
      (`self.SetOrderUi` _returnvalue)
      (`PanelWidget.AddChild` _asborder _returnvalue)
      (return))))

(fn `SubmitDish`
  (params (Dish_Name :type String))
  (returns (bIsSuccess :type Boolean) (Score :type Integer))
  (return false 0))

(fn `UserConstructionScript`)