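; Base Blueprint for world items that an interactor can pick up.
; On interact press, it turns off physics and collision on its static mesh, then passes its item data and itself to the interactor through a GiveItem message.
; Tick destroys the actor once it falls below a fixed height.
; Its own GiveItem and TakeItem functions are stubs that return false.
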(event `self.ReceiveTick`
  (params (DeltaSeconds :type "Float (single-precision)"))
  (bind (_returnvalue_x _returnvalue_y _returnvalue_z) (`KismetMathLibrary.BreakVector` (`self.K2_GetActorLocation`)))
  (if (< _returnvalue_z -100.0)
    (`self.K2_DestroyActor`)))

(event `/Game/Interfaces/BPI_Interactable.InteractPress`
  (params (Interactor :type "Actor Object Reference"))
  (bind _staticmesh (`self.StaticMesh`))
  (`PrimitiveComponent.SetSimulatePhysics` _staticmesh false)
  (`PrimitiveComponent.SetCollisionEnabled` _staticmesh "NoCollision")
  (message `/Game/Interfaces/BPI_ItemHandler.GiveItem` Interactor (`self.ItemData`) self))

(fn `GiveItem`
  (params (ItemInfo :type "/Game/Data/ST_ItemData Structure") (ActorInfo :type "Actor Object Reference"))
  (returns (IsSuccess :type Boolean))
  (return false))

(fn `TakeItem`
  (returns (IsSuccess :type Boolean) (ItemInfo :type "/Game/Data/ST_ItemData Structure") (ActorInfo :type "Actor Object Reference"))
  (return false (struct) null))

(fn `UserConstructionScript`)