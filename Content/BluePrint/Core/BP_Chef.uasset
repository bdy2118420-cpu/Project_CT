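; Player chef character that moves on world axes, boosts to double speed, and carries one item on its head socket.
; E press and release box-trace forward to send interact messages; pressing with nothing hit throws the held item with physics.
; GiveItem and TakeItem handle item handoffs, forwarding to BP_Plate when the held item's name contains "접시" (plate).
; Cut loops a chop animation while walk speed is zero, otherwise restores ABP_Chef.
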(event `InputAction|Boost`
  (params (Key :type "Key Structure"))
  (bind _charactermovement (`self.CharacterMovement`))
  (:`Pressed`
    (set `CharacterMovementComponent.MaxWalkSpeed` (* (`self.WalkSpeed`) 2.0) _charactermovement))
  (:`Released`
    (set `CharacterMovementComponent.MaxWalkSpeed` (`self.WalkSpeed`) _charactermovement)))

(event `InputAxis|MoveFoward`
  (params (AxisValue :type "Float (single-precision)"))
  ; 좌우 이동
  (`self.AddMovementInput` (`KismetMathLibrary.MakeVector` AxisValue)))

(event `InputAxis|MoveSide`
  (params (AxisValue :type "Float (single-precision)"))
  ; 좌우 이동
  (`self.AddMovementInput` (`KismetMathLibrary.MakeVector` 0.0 AxisValue)))

(event `Key|E`
  (params (Key :type "Key Structure"))
  ; 상호작용
  (:`Pressed`
    (set `self.Pressed` true)
    (`self.Interact`))
  (:`Released`
    (set `self.Pressed` false)
    (`self.Interact`)))

(fn `Cut`
  (if (== (`CharacterMovementComponent.MaxWalkSpeed` (`self.CharacterMovement`)) 0.0)
    (`SkeletalMeshComponent.PlayAnimation` (`self.Mesh`) "/Game/Asset/Charactor/PandaCharacterArmature_Chop_Loop.PandaCharacterArmature_Chop_Loop" true)
    (else
      (`SkeletalMeshComponent.SetAnimInstanceClass` (`self.Mesh`) "/Game/Animation/ABP_Chef.ABP_Chef_C"))))

(fn `DropItem`
  (locals (NewLocalVar_0 :type "Transform Structure"))
  (bind (_currentitemdata_itemname _currentitemdata_itemicon _currentitemdata_item3dmodel) (break `/Game/Data/ST_ItemData` (`self.CurrentItemData`)))
  (bind _currenthelditem (`self.CurrentHeldItem`))
  (bind _staticmesh (`/Game/BluePrint/Item/BP_ItemBase.StaticMesh` _currenthelditem))
  (`self.K2_DetachFromActor` (`self.CurrentHeldItem`) "KeepWorld" "KeepWorld" "KeepWorld")
  (set `/Game/BluePrint/Item/BP_ItemBase.ItemData` (`self.CurrentItemData`) _currenthelditem)
  (`StaticMeshComponent.SetStaticMesh` _staticmesh _currentitemdata_item3dmodel)
  (`PrimitiveComponent.SetSimulatePhysics` _staticmesh true)
  (`PrimitiveComponent.SetCollisionProfileName` _staticmesh "PhysicsActor" true)
  (`PrimitiveComponent.AddImpulse` (`/Game/BluePrint/Item/BP_ItemBase.StaticMesh` _currenthelditem) (+ (* (`self.GetActorForwardVector`) (`self.Throwforward`)) (* (`self.GetActorUpVector`) (`self.ThrowUpWard`))) "HeadSocket" true)
  (`SceneComponent.K2_AddLocalRotation` (`Actor.RootComponent` _currenthelditem) (`KismetMathLibrary.RandomRotator` true) false false)
  (set `self.CurrentHeldItem` null)
  (set `self.CurrentItemData` (struct)))

(fn `GiveItem`
  (params (ItemInfo :type "/Game/Data/ST_ItemData Structure") (ActorInfo :type "Actor Object Reference"))
  (returns (IsSuccess :type Boolean))
  (locals (NewLocalVar :type "/Game/Data/ST_ItemData Structure"))
  (bind _currentitemdata_itemname (break `/Game/Data/ST_ItemData` (`self.CurrentItemData`)))
  (if (`KismetStringLibrary.Contains` _currentitemdata_itemname "접시")
    (bind _asbp_plate (cast `/Game/BluePrint/Item/BP_Plate` (`self.CurrentHeldItem`)))
    (bind _issuccess (`/Game/BluePrint/Item/BP_ItemBase.GiveItem` _asbp_plate (`local.ItemInfo`) (`local.ActorInfo`)))
    (return _issuccess)
    (else
      (set `self.CurrentItemData` (`local.ItemInfo`))
      (bind _asbp_item_base (cast `/Game/BluePrint/Item/BP_ItemBase` (`local.ActorInfo`)))
      (set `self.CurrentHeldItem` _asbp_item_base)
      (bind _returnvalue (`self.K2_AttachToComponent` (`self.CurrentHeldItem`) (`self.Mesh`) "HeadSocket" "SnapToTarget" "SnapToTarget" "KeepWorld" true))
      (return _returnvalue))))

(fn `Interact`
  ; 트레이스를 통한 상호작용
  (bind (_outhit _returnvalue) (`KismetSystemLibrary.BoxTraceSingle` (`self.K2_GetActorLocation`) (+ (`self.K2_GetActorLocation`) (* (`self.GetActorForwardVector`) (`self.Interact Range`))) (50.0 50.0 150.0) (struct) "TraceTypeQuery1"))
  (if _returnvalue
    (if (`self.Pressed`)
      (bind (_bblockinghit _binitialoverlap _time _distance _location _impactpoint _normal _impactnormal _physmat _hitactor) (`GameplayStatics.BreakHitResult` _outhit))
      (message `/Game/Interfaces/BPI_Interactable.InteractPress` _hitactor self)
      (else
        (message `/Game/Interfaces/BPI_Interactable.InteractUnPress` _hitactor self)))
    (elif (`self.Pressed`)
      (`/Engine/EditorBlueprintResources/StandardMacros.IsValid` (`self.CurrentHeldItem`)
        (:`Is Valid`
          (`self.DropItem`))))))

(fn `TakeItem`
  (returns (IsSuccess :type Boolean) (ItemInfo :type "/Game/Data/ST_ItemData Structure") (ActorInfo :type "Actor Object Reference"))
  (locals (TempItem :type "Actor Object Reference"))
  ; 머리위에 아이템을 들고있으면 엑터 삭제후 정보 넘겨줌
  (`/Engine/EditorBlueprintResources/StandardMacros.IsValid` (`self.CurrentHeldItem`)
    (:`Is Valid`
      (bind _output_get (set `self.PlateActor` (`self.CurrentHeldItem`)))
      (`self.K2_DetachFromActor` _output_get "KeepRelative" "KeepRelative" "KeepWorld")
      (set `self.CurrentHeldItem` null)
      (set `self.Item Data` (`self.CurrentItemData`))
      (set `self.CurrentItemData` (struct))
      (return true (`self.Item Data`) _output_get))
    (:`Is Not Valid`
      (return false (struct) null))))

(fn `UserConstructionScript`)