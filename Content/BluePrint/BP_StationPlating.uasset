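; BP_StationPlating is a kitchen plating station that holds one item handed over by the interacting chef.
; On interact, a chef carrying an item fills the empty station: it takes the item by message, stores its data and snaps the actor to a counter socket.
; An empty-handed chef receives the stored item and data back through a give-item message, clearing the station.
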(event `/Game/Interfaces/BPI_Interactable.InteractPress`
  (params (Interactor :type "Actor Object Reference"))
  (bind _output_get (set `self.Interactor` Interactor))
  (bind _asbp_chef (cast `/Game/BluePrint/BP_Chef` _output_get))
  (`/Engine/EditorBlueprintResources/StandardMacros.IsValid` (`/Game/BluePrint/BP_Chef.CurrentHeldItem` _asbp_chef)
    (:`Is Valid`
      (`/Engine/EditorBlueprintResources/StandardMacros.IsValid` (`self.HeldItem`)
        (:`Is Not Valid`
          (`self.SpawnActorOnPlating` (`self.Interactor`)))))
    (:`Is Not Valid`
      (`/Engine/EditorBlueprintResources/StandardMacros.IsValid` (`self.HeldItem`)
        (:`Is Valid`
          (message `/Game/Interfaces/BPI_ItemHandler.GiveItem` (`self.Interactor`) (`self.CurrentItemData`) (`self.HeldItem`))
          (set `self.HeldItem` null))))))

(fn `SpawnActorOnPlating`
  (params (Interactor :type "Object Object Reference"))
  (bind (_issuccess _iteminfo _actorinfo) (message `/Game/Interfaces/BPI_ItemHandler.TakeItem` Interactor))
  (set `self.CurrentItemData` _iteminfo)
  (if _issuccess
    (bind _output_get (set `self.HeldItem` _actorinfo))
    (`self.K2_AttachToComponent` _output_get (`self.kitchencounter_innercorner`) "Socket" "SnapToTarget" "SnapToTarget" "SnapToTarget" true)))

(fn `UserConstructionScript`
  (`parent.UserConstructionScript`))