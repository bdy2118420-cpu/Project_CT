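; BP_Chef is the player chef character, handling movement, interaction and carrying one item.
; E press and release run a forward box trace and send press or unpress interact messages to the hit actor.
; GiveItem spawns a BP_ItemBase with the item's mesh on HeadSocket; TakeItem destroys it and returns its data.
; Cut loops a chop animation while walk speed is zero, otherwise restores the ABP_Chef anim class.
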(event `InputAxis|MoveFoward`
  (params (AxisValue :type "Float (single-precision)"))
  ; 좌우 이동
  (`self.AddMovementInput` (`KismetMathLibrary.MakeVector` AxisValue)))

(event `InputAxis|MoveSide`
  (params (AxisValue :type "Float (single-precision)"))
  ; 좌우 이동
  (`self.AddMovementInput` (`KismetMathLibrary.MakeVector` 0.0 AxisValue)))

(event `Key|E`
  (params (Key :type "Key Structure"))
  ; 상호작용
  (:`Pressed`
    (set `self.Pressed` true)
    (`self.Interact`))
  (:`Released`
    (set `self.Pressed` false)
    (`self.Interact`)))

(fn `Cut`
  (if (== (`CharacterMovementComponent.MaxWalkSpeed` (`self.CharacterMovement`)) 0.0)
    (`SkeletalMeshComponent.PlayAnimation` (`self.Mesh`) "/Game/Asset/Charactor/PandaCharacterArmature_Chop_Loop.PandaCharacterArmature_Chop_Loop" true)
    (else
      (`SkeletalMeshComponent.SetAnimInstanceClass` (`self.Mesh`) "/Game/Animation/ABP_Chef.ABP_Chef_C"))))

(fn `GiveItem`
  (params (ItemInfo :type "/Game/Data/ST_ItemData Structure"))
  (returns (IsSuccess :type Boolean))
  (locals (NewLocalVar :type "/Game/Data/ST_ItemData Structure"))
  ; 상호작용시 아이템 받기
  (bind _output_get (set `self.CurrentItemData` ItemInfo))
  (bind _returnvalue (`|SpawnActorFromClass` "/Game/BluePrint/BP_ItemBase.BP_ItemBase_C" (`self.GetTransform`) "Undefined" "MultiplyWithRoot" null null))
  (bind _output_get_2 (set `self.CurrentHeldItem` _returnvalue))
  (`StaticMeshComponent.SetStaticMesh` (`/Game/BluePrint/BP_ItemBase.StaticMesh` _output_get_2) (`.Item3DModel_18_8779E8244BCBF5E4A785AB940C4C2424` (break `/Game/Data/ST_ItemData` _output_get)))
  (bind _returnvalue_2 (`self.K2_AttachToComponent` (`self.CurrentHeldItem`) (`self.Mesh`) "HeadSocket" "SnapToTarget" "KeepWorld" "SnapToTarget" true))
  (return _returnvalue_2))

(fn `Interact`
  ; 트레이스를 통한 상호작용
  (bind (_outhit _returnvalue) (`KismetSystemLibrary.BoxTraceSingle` (`self.K2_GetActorLocation`) (+ (`self.K2_GetActorLocation`) (* (`self.GetActorForwardVector`) (`self.Interact Range`))) (100.0 100.0 150.0) (struct) "TraceTypeQuery1"))
  (if _returnvalue
    (if (`self.Pressed`)
      (bind (_bblockinghit _binitialoverlap _time _distance _location _impactpoint _normal _impactnormal _physmat _hitactor) (`GameplayStatics.BreakHitResult` _outhit))
      (message `/Game/Interfaces/BPI_Interactable.InteractPress` _hitactor self)
      (else
        (message `/Game/Interfaces/BPI_Interactable.InteractUnPress` _hitactor self)))))

(fn `TakeItem`
  (returns (IsSuccess :type Boolean) (ItemInfo :type "/Game/Data/ST_ItemData Structure"))
  (locals (TempItem :type "Actor Object Reference"))
  ; 머리위에 아이템을 들고있으면 엑터 삭제후 정보 넘겨줌
  (`/Engine/EditorBlueprintResources/StandardMacros.IsValid` (`self.CurrentHeldItem`)
    (:`Is Valid`
      (`self.K2_DestroyActor` (`self.CurrentHeldItem`))
      (set `self.CurrentHeldItem` null)
      (return true (`self.CurrentItemData`)))
    (:`Is Not Valid`
      (return false))))

(fn `UserConstructionScript`)