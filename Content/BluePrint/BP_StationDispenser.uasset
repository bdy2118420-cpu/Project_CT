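; Data-driven dispenser station actor that hands an item to whoever interacts with it.
; The construction script uses DispenseID to look up its row in DT_DIspenserData and apply that row's station mesh.
; InteractPress reads the same row's TargetItemID, fetches that item from DT_ItemData and passes it to the interactor through the GiveItem interface message.
; The dispenser's own GiveItem always returns false.
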(event `/Game/Interfaces/BPI_Interactable.InteractPress`
  (params (Interactor :type "Actor Object Reference"))
  ; 상호작용 발생시 자기 자신의 Actor정보를 데이터 테이블에서 찾아 넘겨줌
  (set `self.Interactor` Interactor)
  (bind _returnvalue (`|GetDataTableRow` "/Game/Data/DT_DIspenserData.DT_DIspenserData" (`self.DispenseID`))
    (:`then`
      (bind _returnvalue_2 (`|GetDataTableRow` "/Game/Data/DT_ItemData.DT_ItemData" (`.TargetItemID_9_9878566A4187DF66ADACBC95CD162081` (break `/Game/Data/ST_DIspenserData` _returnvalue)))
        (:`then`
          (message `/Game/Interfaces/BPI_ItemHandler.GiveItem` (`self.Interactor`) _returnvalue_2))))))

(fn `GiveItem`
  (params (ItemInfo :type "/Game/Data/ST_ItemData Structure"))
  (returns (IsSuccess :type Boolean))
  (return false))

(fn `UserConstructionScript`
  ; ID에 따른 Mesh변환
  (`parent.UserConstructionScript`)
  (bind _returnvalue (`|GetDataTableRow` "/Game/Data/DT_DIspenserData.DT_DIspenserData" (`self.DispenseID`))
    (:`then`
      (bind _output_get (set `self.ST_Dispense` _returnvalue))
      (`StaticMeshComponent.SetStaticMesh` (`self.StaticMesh`) (`|ConvertAsset` (`.StationMesh_11_095537A74EC48472C8B823A21282EC04` (break `/Game/Data/ST_DIspenserData` _output_get)))))))