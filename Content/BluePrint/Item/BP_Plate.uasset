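; BP_Plate is a plate that collects given items and combines them into a recipe's output item.
; GiveItem flags the item OnPlate, then SetPlateItem compares the sorted item-name list against each DT_RecipeData row.
; A match spawns the DT_ItemData result on Socket1; otherwise, the item attaches to a numbered socket.
; Combining, like destroying the plate, removes every OnPlate item in the world, not just this plate's.
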(event `self.ReceiveDestroyed`
  (`self.Destroy`))

(fn `Destroy`
  (bind _outactors (`GameplayStatics.GetAllActorsOfClass` "/Game/BluePrint/Item/BP_ItemBase.BP_ItemBase_C"))
  (for _array_element _outactors
    (if (`/Game/BluePrint/Item/BP_ItemBase.OnPlate` _array_element)
      (`self.K2_DestroyActor` _array_element))))

(fn `GiveItem`
  (params (ItemInfo :type "/Game/Data/ST_ItemData Structure") (ActorInfo :type "Actor Object Reference"))
  (returns (IsSuccess :type Boolean))
  (set `self.Item Info` ItemInfo)
  (bind _asbp_item_base (cast `/Game/BluePrint/Item/BP_ItemBase` ActorInfo))
  (set `self.CurrentHeldItem` _asbp_item_base)
  (set `/Game/BluePrint/Item/BP_ItemBase.OnPlate` true (`self.CurrentHeldItem`))
  (`self.SetPlateItem`)
  (return false))

(fn `SetPlateItem`
  (locals (RecipItem :type "Array of String") (Recipdata :type "/Game/Data/ST_Recipe Structure") (RecpName :type Name))
  (bind _item_info_itemname (break `/Game/Data/ST_ItemData` (`self.Item Info`)))
  (`KismetArrayLibrary.Array_Add` (`self.PlateItems`) _item_info_itemname)
  (`/Engine/EditorBlueprintResources/StandardMacros.IncrementInt` (`self.ItemNum`)
    (:`  `
      (`KismetArrayLibrary.SortStringArray` (`self.PlateItems`))
      (bind _outrownames (`DataTableFunctionLibrary.GetDataTableRowNames` "/Game/Data/DT_RecipeData.DT_RecipeData"))
      (for _array_element _outrownames
        (bind _returnvalue (`|GetDataTableRow` "/Game/Data/DT_RecipeData.DT_RecipeData" _array_element)
          (:`then`
            (bind _output_get (set `local.Recipdata` _returnvalue))
            (bind _output_get_2 (set `local.RecipItem` (break `/Game/Data/ST_Recipe` _output_get)))
            (set `local.RecpName` (`KismetStringLibrary.Conv_StringToName` (`.OutputItem_5_E6AE20634EA5909F58B832BF1A9DF584` (break `/Game/Data/ST_Recipe` _output_get))))
            (`KismetArrayLibrary.SortStringArray` _output_get_2)
            (if (`KismetArrayLibrary.Array_Identical` (`self.PlateItems`) (`local.RecipItem`))
              (set `self.TargetItem` (`local.RecpName`))
              (set `self.AbleCook` true)))))
      (if (`self.AbleCook`)
        (bind _returnvalue_2 (`|GetDataTableRow` "/Game/Data/DT_ItemData.DT_ItemData" (`self.TargetItem`))
          (:`then`
            (set `self.Item Info` _returnvalue_2)
            (bind _outactors (`GameplayStatics.GetAllActorsOfClass` "/Game/BluePrint/Item/BP_ItemBase.BP_ItemBase_C"))
            (for _array_element_2 _outactors
              (if (`/Game/BluePrint/Item/BP_ItemBase.OnPlate` _array_element_2)
                (`self.K2_DestroyActor` _array_element_2)))
            (bind _returnvalue_3 (`|SpawnActorFromClass` "/Game/BluePrint/Item/BP_ItemBase.BP_ItemBase_C" (`self.GetTransform`) "Undefined" "MultiplyWithRoot" null null))
            (set `/Game/BluePrint/Item/BP_ItemBase.OnPlate` true _returnvalue_3)
            (bind _output_get_3 (set `/Game/BluePrint/Item/BP_ItemBase.ItemData` (`self.Item Info`) _returnvalue_3))
            (`StaticMeshComponent.SetStaticMesh` (`/Game/BluePrint/Item/BP_ItemBase.StaticMesh` _returnvalue_3) (`.Item3DModel_18_8779E8244BCBF5E4A785AB940C4C2424` (break `/Game/Data/ST_ItemData` _output_get_3)))
            (`self.K2_AttachToComponent` _returnvalue_3 (`self.StaticMesh`) "Socket1" "SnapToTarget" "SnapToTarget" "KeepWorld" true)
            (set `self.ItemNum` 0)
            (set `self.AbleCook` false)
            (return)))
        (else
          (`self.K2_AttachToComponent` (`self.CurrentHeldItem`) (`self.StaticMesh`) (`KismetStringLibrary.Conv_StringToName` (`KismetStringLibrary.Concat_StrStr` "Socket" (`KismetStringLibrary.Conv_IntToString` (`self.ItemNum`)))) "SnapToTarget" "SnapToTarget" "KeepWorld" true)
          (return))))))

(fn `UserConstructionScript`
  (`parent.UserConstructionScript`))