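; BP_Chef is the player-controlled chef pawn, with axis movement and E-key interaction.
; Interact box-traces forward by InteractRange and sends InteractMessage, passing itself, to the hit actor.
; GiveItem stores item data and spawns a BP_ItemBase with that mesh on HeadSocket; TakeItem destroys the held item and returns its data.
; Cut plays the cutting animation once.
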(event `InputAxis|MoveFoward`
  (params (AxisValue :type "Float (single-precision)"))
  ; 좌우 이동
  (`self.AddMovementInput` (`KismetMathLibrary.MakeVector` AxisValue)))

(event `InputAxis|MoveSide`
  (params (AxisValue :type "Float (single-precision)"))
  ; 좌우 이동
  (`self.AddMovementInput` (`KismetMathLibrary.MakeVector` 0.0 AxisValue)))

(event `Key|E`
  (params (Key :type "Key Structure"))
  ; 상호작용
  (:`Pressed`
    (`self.Interact`)))

(fn `Cut`
  (`SkeletalMeshComponent.PlayAnimation` (`self.Mesh`) "/Game/Project/Animation/AM_Cut.AM_Cut" false))

(fn `GiveItem`
  (params (ItemInfo :type "/Game/Project/Data/ST_ItemData Structure"))
  (returns (IsSuccess :type Boolean))
  (locals (NewLocalVar :type "/Game/Project/Data/ST_ItemData Structure"))
  ; 상호작용시 아이템 받기
  (bind _output_get (set `self.CurrentItemData` ItemInfo))
  (bind _returnvalue (`|SpawnActorFromClass` "/Game/Project/BluePrint/BP_ItemBase.BP_ItemBase_C" (`self.GetTransform`) "Undefined" "MultiplyWithRoot" null null))
  (bind _output_get_2 (set `self.CurrentHeldItem` _returnvalue))
  (`StaticMeshComponent.SetStaticMesh` (`/Game/Project/BluePrint/BP_ItemBase.StaticMesh` _output_get_2) (`|ConvertAsset` (`.Item3DModel_13_8779E8244BCBF5E4A785AB940C4C2424` (break `/Game/Project/Data/ST_ItemData` _output_get))))
  (bind _returnvalue_2 (`self.K2_AttachToComponent` (`self.CurrentHeldItem`) (`self.Mesh`) "HeadSocket" "SnapToTarget" "KeepWorld" "SnapToTarget" true))
  (return _returnvalue_2))

(fn `Interact`
  ; 트레이스를 통한 상호작용
  (bind (_outhit _returnvalue) (`KismetSystemLibrary.BoxTraceSingle` :`Start` (`self.K2_GetActorLocation`) :`End` (+ (`self.K2_GetActorLocation`) (* (`self.GetActorForwardVector`) (`self.Interact Range`))) :`HalfSize` (100.0 100.0 150.0) :`TraceChannel` "TraceTypeQuery1" :`DrawDebugType` "ForDuration"))
  (if _returnvalue
    (message `/Game/Project/Interfaces/BPI_Interactable.Interact` (`.HitActor` (`GameplayStatics.BreakHitResult` _outhit)) self)))

(fn `TakeItem`
  (returns (IsSuccess :type Boolean) (ItemInfo :type "/Game/Project/Data/ST_ItemData Structure"))
  (locals (TempItem :type "Actor Object Reference"))
  ; 머리위에 아이템을 들고있으면 엑터 삭제후 정보 넘겨줌
  (`/Engine/EditorBlueprintResources/StandardMacros.IsValid` (`self.CurrentHeldItem`)
    (:`Is Valid`
      (`self.K2_DestroyActor` (`self.CurrentHeldItem`))
      (set `self.CurrentHeldItem` null)
      (return true (`self.CurrentItemData`)))
    (:`Is Not Valid`
      (return false))))

(fn `UserConstructionScript`)