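; Cooking station counter, set up as a cutting board, where a chef places a carried item and cuts it.
; Interacting while empty takes the Interactor's item and spawns a BP_ItemBase with its mesh at the FoodCounter socket.
; Interacting while loaded scans DT_RecipeData by item and StationID, then starts the chef's cut.
; A cooking-time timer restores ABP_Chef; the output item is unused and IsProcessing is never cleared here.
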(event `self.ReceiveBeginPlay`
  (`parent.ReceiveBeginPlay`))

(event `/Game/Project/Interfaces/BPI_Interactable.Interact`
  (params (Interactor :type "Actor Object Reference"))
  (set `self.Interactor` Interactor)
  ; 도마에 아이템이 없을때
  (`/Engine/EditorBlueprintResources/StandardMacros.IsValid` (`self.HeldItem`)
    (:`Is Valid`
      ; 도마에 아이템이 있고 작업중이 아닐때
      (if (not (`self.IsProcessing`))
        ; 도마 작업이 가능한지 검증
        (bind (_outputitem _cookingtime) (`self.FindRecipe`))
        (set `self.IsProcessing` true)
        (bind _asbp_chef (cast `/Game/Project/BluePrint/BP_Chef` (`self.Interactor`)))
        (`/Game/Project/BluePrint/BP_Chef.Cut` _asbp_chef)
        (`KismetSystemLibrary.K2_SetTimerDelegate` (delegate `CustomEvent`) _cookingtime)))
    (:`Is Not Valid`
      ; 도마위의 없으면 머리위의 아이템 소환
      (`self.SpawnActorOnCutBoard` (`self.Interactor`)))))

(event `CustomEvent`
  (`SkeletalMeshComponent.SetAnimInstanceClass` (`Character.Mesh` (stale `/Game/Project/Interfaces/BPI_Interactable.Interact` _asbp_chef)) "/Game/Project/Animation/ABP_Chef.ABP_Chef_C"))

(fn `FindRecipe`
  (returns (OutputItem :type String) (Cookingtime :type "Float (double-precision)"))
  (locals (NewLocalVar :type "Array of Name"))
  (bind _currentitemdata_itemname (break `/Game/Project/Data/ST_ItemData` (`self.CurrentItemData`)))
  (bind _outrownames (`DataTableFunctionLibrary.GetDataTableRowNames` "/Game/Project/Data/DT_RecipeData.DT_RecipeData"))
  (bind _output_get (set `local.NewLocalVar` _outrownames))
  (for _array_element _output_get
    (bind _returnvalue (`|GetDataTableRow` "/Game/Project/Data/DT_RecipeData.DT_RecipeData" _array_element)
      (:`then`
        (if (and (`KismetArrayLibrary.Array_Contains` (break `/Game/Project/Data/ST_Recipe` _returnvalue) _currentitemdata_itemname) (== (`.RequiredStation_15_995D9C9146BBD48278CB90BE966B2076` (break `/Game/Project/Data/ST_Recipe` _returnvalue)) (`self.StationID`)))
          (return (`.OutputItem_5_E6AE20634EA5909F58B832BF1A9DF584` (break `/Game/Project/Data/ST_Recipe` _returnvalue)) (`.Cookingtime_11_9CDD3667464780268DD0E387204BF1B4` (break `/Game/Project/Data/ST_Recipe` _returnvalue))))))))

(fn `SpawnActorOnCutBoard`
  (params (Interactor :type "Object Object Reference"))
  ; 머리에 있는 아이템정보 가져오기
  (bind (_issuccess _iteminfo) (message `/Game/Project/Interfaces/BPI_ItemHandler.TakeItem` Interactor))
  (set `self.CurrentItemData` _iteminfo)
  (if _issuccess
    ; 도마 위에 소환
    (bind _returnvalue (`|SpawnActorFromClass` "/Game/Project/BluePrint/BP_ItemBase.BP_ItemBase_C" (`SceneComponent.GetSocketTransform` (`self.StaticMesh`) "FoodCounter" "RTS_World") "Undefined" "MultiplyWithRoot" null null))
    (set `self.HeldItem` _returnvalue)
    ; 매쉬 설정
    (`StaticMeshComponent.SetStaticMesh` (`/Game/Project/BluePrint/BP_ItemBase.StaticMesh` _returnvalue) (`|ConvertAsset` (`.Item3DModel_13_8779E8244BCBF5E4A785AB940C4C2424` (break `/Game/Project/Data/ST_ItemData` _iteminfo))))))

(fn `UserConstructionScript`
  (`parent.UserConstructionScript`))